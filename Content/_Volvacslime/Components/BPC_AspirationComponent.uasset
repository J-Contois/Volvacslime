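; Actor component that lets its owner suck in a detected object, like a vacuum, and hold it in its mouth.
; The target detection component supplies the candidate, and StartAspiration checks that the mouth is empty and the target accepts the aspiration strength.
; While active, tick pulls the target's mesh by force toward a tagged TransferPoint, or the root as fallback.
; Within the absorb threshold, it notifies the target, marks the mouth full and disables tick.
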(event `self.ReceiveBeginPlay`
  (bind _returnvalue (`self.GetOwner`))
  (bind _output (`|GetArrayItem` (`Actor.GetComponentsByTag` (`self.OwnerActor`) "/Script/Engine.SceneComponent" "TransferPoint")))
  (set `self.OwnerActor` _returnvalue)
  (bind _output_get (set `self.DetectionComp` (`Actor.GetComponentByClass` _returnvalue "/Game/_Volvacslime/Components/BPC_TargetDetectionComponent.BPC_TargetDetectionComponent_C")))
  (add `/Game/_Volvacslime/Components/BPC_TargetDetectionComponent.OnTargetChanged` _output_get (delegate `HandleTargetChanged`))
  (`/Engine/EditorBlueprintResources/StandardMacros.IsValid` _output
    (:`Is Valid`
      (set `self.TransferPoint` _output))
    (:`Is Not Valid`
      (set `self.TransferPoint` (`Actor.RootComponent` (`self.GetOwner`))))))

(event `HandleTargetChanged`
  (params (NewTarget :type "Actor Object Reference"))
  (set `self.PotentialTarget` NewTarget))

(event `self.ReceiveTick`
  (params (DeltaSeconds :type "Float (single-precision)"))
  (bind _returnvalue (`SceneComponent.K2_GetComponentLocation` (`self.TransferPoint`)))
  (bind _returnvalue_2 (`Actor.K2_GetActorLocation` (`self.PotentialTarget`)))
  (if (or (not (`self.bIsAspirating`)) (not (`KismetSystemLibrary.IsValid` (`self.PotentialTarget`))))
    (`self.StopAspiration`)
    (elif (< (`KismetMathLibrary.Vector_Distance` _returnvalue _returnvalue_2) (`self.AbsorbThreshold`))
      (message `/Game/_Volvacslime/Interfaces/BPI_Interactable.OnAspirated` (`self.PotentialTarget`) (`self.OwnerActor`))
      (set `self.bHasItemInMouth` true)
      (`self.StopAspiration`)
      (else
        (`PrimitiveComponent.AddForce` (`Actor.GetComponentByClass` (`self.PotentialTarget`) "/Script/Engine.StaticMeshComponent") (* (`KismetMathLibrary.Normal` (- _returnvalue _returnvalue_2)) (`self.PullForce`)) "None" true)))))

(fn `StartAspiration`
  (bind _potentialtarget (`self.PotentialTarget`))
  (if (`self.bHasItemInMouth`)
    (return)
    (else
      (`/Engine/EditorBlueprintResources/StandardMacros.IsValid` _potentialtarget
        (:`Is Valid`
          (bind _bisaspirated (message `/Game/_Volvacslime/Interfaces/BPI_Interactable.CanBeAspirated` _potentialtarget (`self.AspirationStregth`)))
          (if _bisaspirated
            (set `self.bIsAspirating` true)
            (`self.SetComponentTickEnabled` true)
            (else
              (`KismetSystemLibrary.PrintString` "Trop lourd !")
              (return))))))))

(fn `StopAspiration`
  (set `self.bIsAspirating` false)
  (`self.SetComponentTickEnabled` false))