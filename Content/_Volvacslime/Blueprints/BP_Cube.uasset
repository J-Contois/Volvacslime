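; BP_Cube is a cube actor that appears to test overlap with the Volvacslime player's target detection sphere.
; When the player overlaps the Cube component, it caches the cast character reference once.
; It then prints a debug message if the overlapping component is that character's DetectionSphere.
; CanBeAspirated always returns false, while GetInteractableData and GetPlayerRef are empty stubs.
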(event `self.ReceiveBeginPlay`)

(event `self.Cube.OnComponentBeginOverlap`
  (params (OverlappedComponent :type "PrimitiveComponent Object Reference") (OtherActor :type "Actor Object Reference") (OtherComp :type "PrimitiveComponent Object Reference") (OtherBodyIndex :type Integer) (bFromSweep :type Boolean) (SweepResult :type "HitResult Structure (by ref)"))
  (if (== OtherActor (`GameplayStatics.GetPlayerCharacter` 0))
    (`|ExecutionSequence`
      (:`then_0`
        (`/Engine/EditorBlueprintResources/StandardMacros.DoOnce` false
          (:`Completed`
            (bind _output_get (set `self.PlayerActor` OtherActor))
            (bind _asbp_volvacslime_character (cast `/Game/_Volvacslime/00_Core/Blueprints/BP_VolvacslimeCharacter` _output_get))
            (set `self.As BP Volvacslime Character` _asbp_volvacslime_character))))
      (:`then_1`
        (if (== (`/Game/_Volvacslime/Blueprints/BPC_TargetDetectionComponent.DetectionSphere` (`/Game/_Volvacslime/00_Core/Blueprints/BP_VolvacslimeCharacter.BPC_TargetDetectionComponent` (`self.As BP Volvacslime Character`))) OtherComp)
          (`KismetSystemLibrary.PrintString` "Hello"))))))

(fn `CanBeAspirated`
  (params (RequesterStrenght :type "Float (double-precision)"))
  (returns (IsAspirated :type Boolean))
  (return false))

(fn `GetInteractableData`
  (returns (S_InteractableData :type "/Game/_Volvacslime/Data/S_InteractableData Structure"))
  (return))

(fn `GetPlayerRef`
  (returns (`Player Ref` :type "/Game/_Volvacslime/00_Core/Blueprints/BP_VolvacslimeCharacter Object Reference"))
  (return null))

(fn `UserConstructionScript`)