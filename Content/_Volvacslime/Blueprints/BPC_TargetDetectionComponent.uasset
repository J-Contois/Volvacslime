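; Actor component that detects nearby BPI_Interactable actors and picks a current target to highlight for its owner.
; A detection sphere created at BeginPlay maintains the candidate list through overlap events.
; A looping timer filters candidates by forward-vector dot product, then scores them by weighted angle and distance.
; Target updates toggle highlights through interface messages and fire OnTargetChanged.
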(event `self.ReceiveBeginPlay`
  (bind _detectionsphere (`self.DetectionSphere`))
  (bind _output_get (set `self.OwnerActor` (`self.GetOwner`)))
  (bind _returnvalue (`|AddComponentByClass` :`self` _output_get :`Class` "/Script/Engine.SphereComponent"))
  (set `self.DetectionSphere` _returnvalue)
  (`PrimitiveComponent.SetCollisionProfileName` _detectionsphere "OverlapAllDynamic" true)
  (`SphereComponent.SetSphereRadius` _detectionsphere (`self.DetectionRadius`) true)
  (set `PrimitiveComponent.bGenerateOverlapEvents` true _detectionsphere)
  (add `PrimitiveComponent.OnComponentBeginOverlap` _detectionsphere (delegate `HandleBeginOverlap`))
  (add `PrimitiveComponent.OnComponentEndOverlap` _detectionsphere (delegate `HandleEndOverlap`))
  (`KismetSystemLibrary.K2_SetTimer` null "EvaluateBestTarget" (`self.EvaluateInterval`) true))

(event `HandleEndOverlap`
  (params (OverlappedComponent :type "PrimitiveComponent Object Reference") (OtherActor :type "Actor Object Reference") (OtherComp :type "PrimitiveComponent Object Reference") (OtherBodyIndex :type Integer))
  (`KismetArrayLibrary.Array_RemoveItem` (`self.CandidateActors`) OtherActor)
  (if (== OtherActor (`self.CurrentTarget`))
    (if (`KismetSystemLibrary.DoesImplementInterface` OtherActor "/Game/_Volvacslime/Blueprints/Interaction/BPI_Interactable.BPI_Interactable_C")
      (message `/Game/_Volvacslime/Blueprints/Interaction/BPI_Interactable.SetHighlighted` OtherActor false)
      (set `self.CurrentTarget` null)
      (`self.OnTargetChanged` null))))

(event `HandleBeginOverlap`
  (params (OverlappedComponent :type "PrimitiveComponent Object Reference") (OtherActor :type "Actor Object Reference") (OtherComp :type "PrimitiveComponent Object Reference") (OtherBodyIndex :type Integer) (bFromSweep :type Boolean) (SweepResult :type "HitResult Structure (by ref)"))
  (if (`KismetSystemLibrary.DoesImplementInterface` OtherActor "/Game/_Volvacslime/Blueprints/Interaction/BPI_Interactable.BPI_Interactable_C")
    (`KismetArrayLibrary.Array_AddUnique` (`self.CandidateActors`) OtherActor)))

(fn `CalculateScore`
  (params (Dot :type "Float (double-precision)") (Dist :type "Float (double-precision)"))
  (returns (Score :type "Float (double-precision)"))
  (return (+ (* Dot (`self.AngleWeight`)) (* (- 1.0 (`KismetMathLibrary.FClamp` (/ Dist (`self.DetectionRadius`)))) (`self.DistanceWeight`)))))

(fn `EvaluateBestTarget`
  (locals (BestActor :type "Actor Object Reference") (BestScore :type "Float (double-precision)" :default -1.0))
  (for _array_element (`self.CandidateActors`)
    (`/Engine/EditorBlueprintResources/StandardMacros.IsValid` _array_element
      (:`Is Valid`
        (bind _returnvalue (`KismetMathLibrary.Dot_VectorVector` (`Actor.GetActorForwardVector` (`self.OwnerActor`)) (`KismetMathLibrary.Normal` (- (`Actor.K2_GetActorLocation` _array_element) (`Actor.K2_GetActorLocation` (`self.OwnerActor`))))))
        (if (< _returnvalue (`self.MinDotProduct`))
          (bind _score (`self.CalculateScore` _returnvalue (`Actor.GetDistanceTo` (`self.OwnerActor`) _array_element)))
          (if (> _score (`local.BestScore`))
            (set `local.BestScore` _score)
            (set `local.BestActor` _array_element))))))
  (`self.SetTarget` (`local.BestActor`)))

(fn `SetTarget`
  (params (NewTarget :type "Actor Object Reference"))
  (`/Engine/EditorBlueprintResources/StandardMacros.IsValid` (`self.CurrentTarget`)
    (:`Is Valid`
      (message `/Game/_Volvacslime/Blueprints/Interaction/BPI_Interactable.SetHighlighted` (`self.CurrentTarget`) false)
      (set `self.CurrentTarget` NewTarget)
      (`/Engine/EditorBlueprintResources/StandardMacros.IsValid` NewTarget
        (:`Is Valid`
          (message `/Game/_Volvacslime/Blueprints/Interaction/BPI_Interactable.SetHighlighted` NewTarget true)
          (`self.OnTargetChanged` NewTarget))))))