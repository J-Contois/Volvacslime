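; BP_PhysicsObject_Base is a physics object that can be sucked up (aspirated) by a requester, named as a base class for such interactables.
; CanBeAspirated compares the requester's strength to RequiredStrength, and GetInteractableData returns its ItemData.
; OnAspirated stops physics on the Cube, then hides the actor and disables its collision rather than destroying it.
; SetHighlighted and OnExpelled are empty stubs, so nothing here restores an aspirated object.
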(event `/Game/_Volvacslime/Interfaces/BPI_Interactable.SetHighlighted`
  (params (bHighlighted :type Boolean)))

(event `/Game/_Volvacslime/Interfaces/BPI_Interactable.OnAspirated`
  (params (Instigator :type "Actor Object Reference"))
  (`PrimitiveComponent.SetSimulatePhysics` (`self.Cube`) false)
  (`self.SetActorHiddenInGame` true)
  (`self.SetActorEnableCollision` false))

(event `/Game/_Volvacslime/Interfaces/BPI_Interactable.OnExpelled`
  (params (Instigator :type "Actor Object Reference") (LauchVelocity :type "Vector Structure")))

(fn `CanBeAspirated`
  (params (RequesterStrenght :type "Float (double-precision)"))
  (returns (bIsAspirated :type Boolean))
  (return (>= RequesterStrenght (`self.RequiredStrength`))))

(fn `GetInteractableData`
  (returns (S_InteractableData :type "/Game/_Volvacslime/Data/S_InteractableData Structure"))
  (return (`self.ItemData`)))

(fn `UserConstructionScript`)